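; WebSocket actor that connects the Tic Tac Tie game to a local matchmaking server.
; On BeginPlay it registers itself with TicTacTie_GameMode, failing fatally if the game mode has the wrong type.
; SearchGame opens the socket, sends the username once connected, prints an "OK" reply and forwards any other message through the OnError dispatcher.
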(event `self.ReceiveBeginPlay`
  (bind _astic_tac_tie_game_mode (cast `/Game/Blueprints/TicTacTie_GameMode` (`GameplayStatics.GetGameMode`))
    (:`then`
      (set `/Game/Blueprints/TicTacTie_GameMode.WebSocket` self _astic_tac_tie_game_mode))
    (:`CastFailed`
      (`Log.Fatal` "Game mode has wrong type"))))

(event `SearchGame`
  (params (Username :type String))
  ;[1 1 1] Connect to server
  (`self.CreateWebSocket` "ws://localhost:8080")
  (`self.Connect`)
  (add `self.OnConnectedEvent` (delegate `OnConnect`))
  (add `self.OnMessageEvent` (delegate `OnMessage`)))

(event `OnConnect`
  ;[1 1 1] Send username if connected
  (`self.Send` (stale `SearchGame` Username)))

(event `OnMessage` :!signature `self.OnMessageEvent`
  (params (MessageString :type String))
  (if (`KismetStringLibrary.EqualEqual_StrStr` MessageString "OK")
    (`KismetSystemLibrary.PrintString` MessageString)
    (else
      (`self.OnError` MessageString))))

(fn `UserConstructionScript`)